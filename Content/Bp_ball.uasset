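; Bp_ball is a ball actor that moves in a straight line along its Direction at Speed and bounces off whatever it hits.
; Each tick it applies a swept local offset, and on a blocking hit reflects Direction about the surface normal, flattened to the XY plane.
; Each bounce also prints Speed and reduces it by a fixed Deceleration, a tenth of the starting speed set at BeginPlay, down to MinSpeed.
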(event `self.ReceiveBeginPlay`
  (set `self.Deceleration` (* (`self.speed`) 0.1)))

(event `self.ReceiveTick`
  (params (DeltaSeconds :type "Float (single-precision)"))
  (bind _speed (`self.speed`))
  (bind _sweephitresult (`self.K2_AddActorLocalOffset` (* (* (`self.direction`) (`self.speed`)) DeltaSeconds) true))
  (bind (_bblockinghit _binitialoverlap _time _distance _location _impactpoint _normal) (`GameplayStatics.BreakHitResult` _sweephitresult))
  (if _bblockinghit
    (bind (_returnvalue_x _returnvalue_y) (`KismetMathLibrary.BreakVector` (`KismetMathLibrary.GetReflectionVector` (`self.direction`) _normal)))
    (set `self.direction` (`KismetMathLibrary.MakeVector` _returnvalue_x _returnvalue_y))
    (`KismetSystemLibrary.PrintString` (`KismetStringLibrary.Conv_DoubleToString` _speed))
    (set `self.speed` (`KismetMathLibrary.FMax` (- _speed (`self.Deceleration`)) (`self.min_speed`)))))

(fn `UserConstructionScript`)